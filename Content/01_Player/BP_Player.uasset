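; Player character with cursor-based aiming, firing projectiles from a switchable pencil (Lapiz) or eraser (Goma) weapon.
; Enhanced Input drives movement, jumping, shooting and BP_Door interaction; Tick yaws the actor toward the cursor hit.
; Number keys swap the weapon mesh and type, which selects the bullet class spawned.
; It creates reticule and HUD widgets, toggles pause on Backspace, and ReceiveDamage updates health, showing WBP_Reprobado and destroying itself at zero.
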(event Input|EnhancedActionEvents|EnhancedInputActionIA_MOVE
  (params (ActionValue :type Vector%202D%20Structure) (ElapsedSeconds :type Float%20%28double-precision%29) (TriggeredSeconds :type Float%20%28double-precision%29) (InputAction :type Input%20Action%20Object%20Reference :default "/Game/02_Mapping/IA_MOVE.IA_MOVE"))
  (Pawn|Input|AddMovementInput (Math|Vector|GetRightVector (Math|Rotator|MakeRotator 0.0 0.0 (.yaw (Pawn|GetControlRotation :!class /Script/Engine.Pawn)))) (.x ActionValue) false)
  (Pawn|Input|AddMovementInput (Math|Vector|GetForwardVector (Math|Rotator|MakeRotator 0.0 0.0 (.yaw (Pawn|GetControlRotation :!class /Script/Engine.Pawn)))) (.y ActionValue) false))

(event Input|EnhancedActionEvents|EnhancedInputActionIA_JUMP
  (params (ActionValue :type Boolean) (ElapsedSeconds :type Float%20%28double-precision%29) (TriggeredSeconds :type Float%20%28double-precision%29) (InputAction :type Input%20Action%20Object%20Reference :default "/Game/02_Mapping/IA_JUMP.IA_JUMP"))
  (:Triggered
    (Character|Jump))
  (:Completed
    (Character|StopJumping)))

(event Input|EnhancedActionEvents|EnhancedInputActionIA_SHOOT
  (params (ActionValue :type Boolean) (ElapsedSeconds :type Float%20%28double-precision%29) (TriggeredSeconds :type Float%20%28double-precision%29) (InputAction :type Input%20Action%20Object%20Reference :default "/Game/02_Mapping/IA_SHOOT.IA_SHOOT"))
  (bind _returnvalue (Transformation|GetActorForwardVector))
  (bind _returnvalue_2 (Transformation|GetActorTransform))
  (bind (_location _rotation) (Math|Transform|BreakTransform _returnvalue_2))
  (bind _returnvalue_3 (* _returnvalue 1e+02))
  (bind (_roll _pitch _yaw) (Math|Rotator|BreakRotator _rotation))
  (bind _returnvalue_4 (+ _location _returnvalue_3))
  (bind _returnvalue_5 (Math|Rotator|MakeRotator _roll 0.0 _yaw))
  (bind _returnvalue_6 (Math|Transform|MakeTransform _returnvalue_4 _returnvalue_5))
  ;[0.15 0.15 0.15 0.5] Disparo shoot
  (switch Utilities|FlowControl|Switch|SwitchonE_weapon (Variables|Default|GetArmaEquipada)
    (:NewEnumerator1
      (Game|SpawnActorfromClass "/Game/05_Blueprints/PLayer/BP_Bullet.BP_Bullet_C" _returnvalue_6 "AlwaysSpawn" "MultiplyWithRoot" 0 0)
      ;[0.15 0.15 0.15 0.5] Sonidos
      (Audio|PlaySound2D "/Game/Sounds/shoot.shoot" 1.0 1.0 0.0 0 0))
    (:NewEnumerator2
      (Game|SpawnActorfromClass "/Game/05_Blueprints/PLayer/BP_Bullet2.BP_Bullet2_C" _returnvalue_6 "AlwaysSpawn" "MultiplyWithRoot" 0 0)
      (Audio|PlaySound2D "/Game/Sounds/shoot.shoot" 1.0 1.0 0.0 0 0))))

(event Input|EnhancedActionEvents|EnhancedInputActionIA_INTERACT
  (params (ActionValue :type Boolean) (ElapsedSeconds :type Float%20%28double-precision%29) (TriggeredSeconds :type Float%20%28double-precision%29) (InputAction :type Input%20Action%20Object%20Reference :default "/Game/02_Mapping/IA_INTERACT.IA_INTERACT"))
  (bind _overlappingactors (Collision|GetOverlappingActors "/Game/05_Blueprints/BP_Door.BP_Door_C" :!class /Script/Engine.Actor))
  (if (> (Utilities|Array|Length _overlappingactors) 0)
    (bind _asbp_door (Utilities|Casting|CastToBP_Door (Utilities|Array|Get(acopy) _overlappingactors)))
    (if (Variables|/Game/05_Blueprints/BP_Door.BP_Door_C|GetJugadorenArea _asbp_door)
      (Default|InteractuarConPuerta _asbp_door self))))

(event EventBeginPlay
  (bind _asbp_playercontroller (Utilities|Casting|CastToBP_PLAYERCONTROLLER (Pawn|GetController)))
  (Utilities|IsValid (PlayerController|LocalPlayerSubsystems|GetEnhancedInputLocalPlayerSubsystem _asbp_playercontroller)
    (:Is%20Valid
      (Input|AddMappingContext (PlayerController|LocalPlayerSubsystems|GetEnhancedInputLocalPlayerSubsystem _asbp_playercontroller) "/Game/02_Mapping/IMC_PLAYER.IMC_PLAYER" 0 "(bIgnoreAllPressedKeysUntilRelease=True,bForceImmediately=False,bNotifyUserSettings=False)")
      (bind _returnvalue (UserInterface|CreateWidget "/Game/03_UI/WBP_RETICULE.WBP_RETICULE_C"))
      (UserInterface|Viewport|AddtoViewport _returnvalue 0)
      (bind _returnvalue_2 (UserInterface|CreateWidget "/Game/03_UI/WBP_HUD.WBP_HUD_C"))
      (bind _output_get (Variables|Default|SetMyHUD _returnvalue_2))
      (UserInterface|Viewport|AddtoViewport _output_get 0))))

(event EventTick
  (params (DeltaSeconds :type Float%20%28single-precision%29))
  (bind _returnvalue (Game|GetPlayerController 0))
  (bind (_hitresult _returnvalue_2) (Game|Player|GetHitResultUnderCursorbyChannel _returnvalue "TraceTypeQuery1" true))
  ;[0.15 0.15 0.15 0.5] esto es para girar el personaje
  (if _returnvalue_2
    (Transformation|SetActorRotation (Math|Rotator|MakeRotator 0.0 0.0 (.yaw (Math|Rotator|FindLookatRotation (Transformation|GetActorLocation) (.Location (Collision|BreakHitResult _hitresult))))))))

(event Input|KeyboardEvents|2
  (params (Key :type Key%20Structure :default "None"))
  (:Pressed
    (CallFunction|ActualizarVisualArma "NewEnumerator2")))

(event Input|KeyboardEvents|1
  (params (Key :type Key%20Structure :default "None"))
  (:Pressed
    (CallFunction|ActualizarVisualArma "NewEnumerator1")))

(event Input|KeyboardEvents|Backspace
  (params (Key :type Key%20Structure :default "None"))
  ;[0.15 0.15 0.15 0.5] Pausar el juego
  (:Pressed
    (Utilities|FlowControl|FlipFlop
      (:A
        (Audio|PlaySound2D "/Game/Sounds/Pausa.Pausa" 1.0 1.0 0.0 0 0)
        (bind _returnvalue (UserInterface|CreateWidget "/Game/03_UI/WBP_Pause.WBP_Pause_C"))
        (UserInterface|Viewport|AddtoViewport _returnvalue 0)
        (Game|SetGamePaused true))
      (:B
        (Audio|PlaySound2D "/Game/Sounds/Despausa.Despausa" 1.0 1.0 0.0 0 0)
        (Widget|RemovefromParent _returnvalue)
        (Game|SetGamePaused false)))))

(fn ConstructionScript)

(fn ReceiveDamage
  (params (DamageAmounts :type Float%20%28double-precision%29))
  (bind _output_get (Variables|Default|SetCurrenthealth (- (Variables|Default|GetCurrenthealth) DamageAmounts)))
  (Default|UpdateHealthBar (Variables|Default|GetMyHUD) (/ _output_get (Variables|Default|GetMaxHealth)))
  (if (<= _output_get 0.0)
    (bind _returnvalue (UserInterface|CreateWidget "/Game/03_UI/WBP_Reprobado.WBP_Reprobado_C"))
    (UserInterface|Viewport|AddtoViewport _returnvalue 0)
    (Actor|DestroyActor)))

(fn ActualizarVisualArma
  (params (NuevaArma :type E_weapon%20Enum :default "NewEnumerator0"))
  (Development|PrintString "actualiz")
  (switch Utilities|FlowControl|Switch|SwitchonE_weapon NuevaArma
    (:NewEnumerator1
      (Components|StaticMesh|SetStaticMesh (Variables|Default|GetMallaarma) "/Game/01_Player/MESH/Weapon/Lapiz.Lapiz")
      (Variables|Default|SetArmaEquipada NuevaArma))
    (:NewEnumerator2
      (Components|StaticMesh|SetStaticMesh (Variables|Default|GetMallaarma) "/Game/01_Player/MESH/Weapon/Goma.Goma")
      (Variables|Default|SetArmaEquipada NuevaArma))))