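; Enemy character that picks one of the first three DT_Enemies rows at random on spawn, setting health, speed and mesh.
; PawnSensing flags sighting of BP_Player in the AI Blackboard.
; AttackPLayer sphere-traces forward, applying the row's damage and playing the combo montage only on a player hit.
; TakeDamage reduces health and, at zero, drops a BP_NumberPickup carrying the row's ValorNumero, prints the enemy name and destroys the actor.
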(event OnSeePawn(PawnSensing)
  (params (Pawn :type Pawn%20Object%20Reference))
  ;[0.15 0.15 0.15 0.5] cambio de boleana en bbdenemy blackboard
  (Utilities|Casting|CastToBP_Player Pawn)
  (AI|Components|Blackboard|SetValueasBool (AI|GetBlackboard (AI|GetAIController self)) (Utilities|Name|MakeLiteralName "HasSeenPlayer?") true))

(event Custom|Attack%20PLayer
  (bind _returnvalue (Transformation|GetActorLocation))
  ;[0.15 0.15 0.15 0.5] Ataque al jugador
  (bind (_outhit _returnvalue_2) (Collision|SphereTraceForObjects _returnvalue (+ _returnvalue (* (Math|Vector|GetForwardVector (Transformation|GetActorRotation)) 2.5e+02)) 1.2e+02 (Utilities|Array|MakeArray "ObjectTypeQuery3") false 0 "ForDuration"))
  (if _returnvalue_2
    (bind _asbp_player (Utilities|Casting|CastToBP_Player (.HitActor (Collision|BreakHitResult _outhit))))
    (Default|ReceiveDamage _asbp_player (.damage (Variables|Default|GetEnemyData)))
    (Animation|PlayAnimMontage "/Game/Variant_Combat/Anims/AM_ComboAttack.AM_ComboAttack" 1.0 "None")))

(event EventBeginPlay
  ;[0.15 0.15 0.15 0.5] Spawn y busqueda de enemigo con vida
  (bind _outrownames (DataTable|GetDataTableRowNames "/Game/06_DataStructure/DT_Enemies.DT_Enemies"))
  (bind _returnvalue (Utilities|GetDataTableRow "/Game/06_DataStructure/DT_Enemies.DT_Enemies" (Utilities|Array|Get(acopy) _outrownames (Math|Random|RandomIntegerinRange 0 2)))
    (:then
      (Variables|Default|SetEnemyData _returnvalue)
      (Variables|Default|SetCurrentHealth (.Maxhealth (Utilities|Struct|BreakS_EnemyData (Variables|Default|GetEnemyData))))
      (Variables|/Script/Engine.CharacterMovementComponent|SetMaxWalkSpeed (Variables|Character|GetCharacterMovement) (.MovSpeed (Utilities|Struct|BreakS_EnemyData (Variables|Default|GetEnemyData))))
      (Components|SkeletalMesh|SetSkeletalMeshAsset (Variables|Character|GetMesh) (.Mesh (Utilities|Struct|BreakS_EnemyData (Variables|Default|GetEnemyData)))))))

(fn ConstructionScript)

(fn TakeDamage
  (bind _returnvalue (Transformation|GetActorTransform))
  (bind _enemydata (Variables|Default|GetEnemyData))
  (bind _output_get (Variables|Default|SetCurrentHealth (- (Variables|Default|GetCurrentHealth) (Variables|Default|GetDamageAmount))))
  (if (<= _output_get 0.0)
    (Game|SpawnActorfromClass "/Game/05_Blueprints/ObjectSpawn/BP_NumberPickup.BP_NumberPickup_C" (Math|Transform|MakeTransform (.location _returnvalue) (.rotation _returnvalue) "1.000000,1.000000,1.000000") "AlwaysSpawn" "MultiplyWithRoot" 0 (.valornumero _enemydata) 0)
    (Development|PrintString (.enemyname _enemydata) true true "(R=1.000000,G=0.137186,B=0.000000,A=1.000000)")
    (Actor|DestroyActor)))