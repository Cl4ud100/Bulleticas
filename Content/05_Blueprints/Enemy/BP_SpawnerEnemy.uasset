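; BP_SpawnerEnemy is an actor that periodically spawns enemies of a configurable class within an area.
; On BeginPlay it starts a looping timer that calls SpawnEnemy at the spawn interval.
; SpawnEnemy spawns one enemy at a random point in the SpawnerEnemyArea bounds, ignoring collisions, only while the world-wide count of that class is below MaxEnemies.
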(event EventBeginPlay
  (Utilities|Time|SetTimerbyFunctionName 0 "SpawnEnemy" (Variables|Default|GetSpawnInterval) true))

(event Collision|EventActorBeginOverlap
  (params (OtherActor :type Actor%20Object%20Reference)))

(event EventTick
  (params (DeltaSeconds :type Float%20%28single-precision%29)))

(fn ConstructionScript)

(fn SpawnEnemy
  (bind _spawnerenemyarea (Variables|Default|GetSpawnerEnemyArea))
  (bind (_origin _boxextent) (Collision|GetComponentBounds _spawnerenemyarea))
  (bind _outactors (Actor|GetAllActorsOfClass (Variables|Default|GetEnemyClass)))
  (if (< (Utilities|Array|Length _outactors) (Variables|Default|GetMaxEnemies))
    (Game|SpawnActorfromClass (Variables|Default|GetEnemyClass) (Math|Transform|MakeTransform (Math|Random|RandomPointinBoundingBox _origin _boxextent)) "AlwaysSpawn" "MultiplyWithRoot" 0 0)))