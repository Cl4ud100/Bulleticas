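; Math-puzzle door that takes the player to the next level when they bring the correct number.
; The first interaction shows the equation on the player's HUD and activates the linked enemy spawner.
; Later interactions compare the player's carried number to the correct result, opening the next level on a match.
; Box overlaps track player presence and toggle a prompt widget.
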(event OnComponentBeginOverlap(Box)
  (params (OverlappedComponent :type Primitive%20Component%20Object%20Reference) (OtherActor :type Actor%20Object%20Reference) (OtherComp :type Primitive%20Component%20Object%20Reference) (OtherBodyIndex :type Integer) (bFromSweep :type Boolean) (SweepResult :type Hit%20Result%20Structure%20%28by%20ref%29))
  (Utilities|Casting|CastToBP_Player OtherActor)
  (Variables|Default|SetJugadorenArea true)
  (Rendering|SetVisibility (Variables|Default|GetAvisoWidget) true false))

(event OnComponentEndOverlap(Box)
  (params (OverlappedComponent :type Primitive%20Component%20Object%20Reference) (OtherActor :type Actor%20Object%20Reference) (OtherComp :type Primitive%20Component%20Object%20Reference) (OtherBodyIndex :type Integer))
  (Utilities|Casting|CastToBP_Player OtherActor)
  (Variables|Default|SetJugadorenArea false)
  (Rendering|SetVisibility (Variables|Default|GetAvisoWidget) false false))

(event Custom|Interactuar%20con%20puerta
  (params (Jugador%20que%20interactua :type Actor%20Object%20Reference))
  (if (Variables|Default|GetbInteraccionporprimeravez)
    (bind _asbp_player (Utilities|Casting|CastToBP_Player Jugador%20que%20interactua))
    (if (== (Variables|/Game/01_Player/BP_Player.BP_Player_C|GetNumeroQueCargo _asbp_player) (Variables|Default|GetResultadoCorrecto))
      (Game|OpenLevel(byName) (Variables|Default|GetSiguiente%20Nivel))
      (Actor|DestroyActor))
    (else
      (Variables|Default|SetbInteraccionporprimeravez true)
      (bind _asbp_player_2 (Utilities|Casting|CastToBP_Player Jugador%20que%20interactua))
      (Default|EcuationUpdate (Variables|/Game/01_Player/BP_Player.BP_Player_C|GetMyHUD _asbp_player_2) (Variables|Default|GetEcuacionActual))
      (Default|ActivarSpawneo (Variables|Default|GetMiSpawnerEnemigos)))))

(fn ConstructionScript)